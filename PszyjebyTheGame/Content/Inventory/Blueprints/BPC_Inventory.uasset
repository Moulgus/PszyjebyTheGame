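; Inventory component for the third-person character that stores items in a sized slot array and handles interaction and inventory UI input.
; BeginPlay adds the input mapping, creates the inventory widget, sizes the array and loads the grid.
; Interact line-traces from the follow camera and messages BPI_Interact actors, passing itself.
; AddToInventory fills the first zero-quantity slot without stacking, while RemoveFromInventory deletes the array element, shrinking the array.
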(event `self.ReceiveBeginPlay`
  (bind _returnvalue (`GameplayStatics.GetPlayerController` 0))
  (`/Engine/EditorBlueprintResources/StandardMacros.IsValid` _returnvalue
    (:`Is Valid`
      (`EnhancedInputSubsystemInterface.AddMappingContext` (pcsubsystem `EnhancedInputLocalPlayerSubsystem` _returnvalue) "/Game/Inventory/Input/IMC_Inventory.IMC_Inventory" 0 (struct))
      (bind _returnvalue_2 (`|CreateWidget` "/Game/Inventory/Widgets/WBP_Inventory.WBP_Inventory_C"))
      (set `self.InventoryWidget` _returnvalue_2)
      (bind _asbp_third_person_character (cast `/Game/ThirdPerson/Blueprints/BP_ThirdPersonCharacter` (`self.GetOwner`)))
      (set `self.BP Third Person Character` _asbp_third_person_character)
      (`KismetArrayLibrary.Array_Resize` (`self.Inventory`) (`self.InventorySize`))
      (`/Game/Inventory/Widgets/WBP_InventoryGrid.LoadInventory` (`/Game/Inventory/Widgets/WBP_Inventory.WBP_InventoryGrid` (`self.InventoryWidget`)) self))))

(event `EnhancedInput|/Game/Inventory/Input/IA_Interact`
  (params (ActionValue :type Boolean) (ElapsedSeconds :type "Float (double-precision)") (TriggeredSeconds :type "Float (double-precision)") (InputAction :type "InputAction Object Reference" :default "/Game/Inventory/Input/IA_Interact.IA_Interact"))
  (bind _followcamera (`/Game/ThirdPerson/Blueprints/BP_ThirdPersonCharacter.FollowCamera` (`self.BP Third Person Character`)))
  (bind _returnvalue (`SceneComponent.K2_GetComponentLocation` _followcamera))
  (:`Started`
    (bind (_outhit _returnvalue_2) (`KismetSystemLibrary.LineTraceSingle` :`Start` _returnvalue :`End` (+ _returnvalue (* (`SceneComponent.GetForwardVector` _followcamera) 1000.0)) :`TraceChannel` "TraceTypeQuery1" :`DrawDebugType` "ForDuration" :`TraceColor` (struct :`R` 1.0 :`G` 0.952062 :`A` 1.0)))
    (bind (_bblockinghit _binitialoverlap _time _distance _location _impactpoint _normal _impactnormal _physmat _hitactor) (`GameplayStatics.BreakHitResult` _outhit))
    (if (and _returnvalue_2 (`KismetSystemLibrary.DoesImplementInterface` _hitactor "/Game/Inventory/Interfaces/BPI_Interact.BPI_Interact_C"))
      (message `/Game/Inventory/Interfaces/BPI_Interact.Interact` _hitactor self))))

(event `EnhancedInput|/Game/Inventory/Input/IA_OpenInventory`
  (params (ActionValue :type Boolean) (ElapsedSeconds :type "Float (double-precision)") (TriggeredSeconds :type "Float (double-precision)") (InputAction :type "InputAction Object Reference" :default "/Game/Inventory/Input/IA_OpenInventory.IA_OpenInventory"))
  (bind _returnvalue (`GameplayStatics.GetPlayerController` 0))
  (:`Started`
    (if (`Widget.IsVisible` (`self.InventoryWidget`))
      (`Widget.RemoveFromParent` (`self.InventoryWidget`))
      (else
        (set `PlayerController.bShowMouseCursor` true _returnvalue)
        (`WidgetBlueprintLibrary.SetInputMode_UIOnlyEx` _returnvalue (`self.InventoryWidget`))
        (`UserWidget.AddToViewport` (`self.InventoryWidget`) 0)))))

(fn `AddToInventory`
  (params (Item :type "/Game/Inventory/Structures/S_ItemMaster Structure (by ref)"))
  (returns (`AddedToInventory?` :type Boolean))
  (for (_array_element _array_index) (`self.Inventory`)
    (if (== (`.Quantity_5_ECA21AC8422A3B7CFB8084ABCB755B5F` (break `/Game/Inventory/Structures/S_ItemMaster` _array_element)) 0)
      (`KismetArrayLibrary.Array_Set` (`self.Inventory`) _array_index (`local.Item`))
      (return true)))
  (return false))

(fn `RemoveFromInventory`
  (params (IndexToRemove :type Integer))
  (`KismetArrayLibrary.Array_Remove` (`self.Inventory`) IndexToRemove))