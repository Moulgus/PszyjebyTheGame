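; BP_PickupActor is a world item that can be picked up into an inventory and highlights when looked at.
; The construction script looks up the ItemData row in its data table to set the static mesh and enable physics simulation.
; Looking at it toggles an overlay material and a widget through Highlight.
; Interact adds ItemData to the passed inventory and, on success, reloads the inventory grid widget and destroys the actor.
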(event `/Game/Inventory/Interfaces/BPI_Interact.Interact`
  (params (Inventory :type "/Game/Inventory/Blueprints/BPC_Inventory Object Reference"))
  (bind _addedtoinventory_ (`/Game/Inventory/Blueprints/BPC_Inventory.AddToInventory` Inventory (`self.ItemData`)))
  (if _addedtoinventory_
    (`/Game/Inventory/Widgets/WBP_InventoryGrid.LoadInventory` (`/Game/Inventory/Widgets/WBP_Inventory.WBP_InventoryGrid` (`/Game/Inventory/Blueprints/BPC_Inventory.InventoryWidget` Inventory)) Inventory)
    (`self.K2_DestroyActor`)))

(event `Highlight`
  (params (`Highlight?` :type Boolean))
  (bind _staticmesh (`self.StaticMesh`))
  (bind _widget (`self.Widget`))
  (if `Highlight?`
    (`MeshComponent.SetOverlayMaterial` _staticmesh "/Game/ThirdPerson/Materials/M_Overlay.M_Overlay")
    (`SceneComponent.SetVisibility` _widget true false)
    (else
      (`MeshComponent.SetOverlayMaterial` _staticmesh null)
      (`SceneComponent.SetVisibility` _widget false false))))

(event `/Game/Inventory/Interfaces/BPI_Interact.LookingAt`
  (params (ShowLookAt :type Boolean))
  (`self.Highlight` ShowLookAt))

(fn `UserConstructionScript`
  (bind (_datatable _rowname) (break `DataTableRowHandle` (`.DataBase_2_3D8CF8D944A50551CD4704BBA03BCA70` (break `/Game/Inventory/Structures/S_ItemMaster` (`self.ItemData`)))))
  (bind _returnvalue (`|GetDataTableRow` _datatable _rowname)
    (:`then`
      (`StaticMeshComponent.SetStaticMesh` (`self.StaticMesh`) (`.StaticMesh_16_8835F9C747145E21A1F55BA76971B416` (break `/Game/Inventory/Structures/S_Item` _returnvalue)))
      (`PrimitiveComponent.SetSimulatePhysics` (`self.StaticMesh`) true))))