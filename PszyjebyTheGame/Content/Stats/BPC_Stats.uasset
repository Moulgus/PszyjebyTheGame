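; Actor component that stores and modifies health, mana and stamina for its owner.
; Increase and decrease functions adjust each current value, capping gains at the matching maximum and flooring mana and stamina at zero.
; Health loss is not clamped and calls the Death dispatcher on every decrease that leaves health at or below zero.
; BeginPlay and Tick are unused, so values change only through these functions.
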(fn `DecreaseHealthPoints`
  (params (Amount :type "Float (double-precision)"))
  (bind _output_get (set `self.CurrentHealthPoints` (- (`self.CurrentHealthPoints`) Amount)))
  (if (<= _output_get 0.0)
    (`self.Death`)))

(fn `DecreaseManaPoints`
  (params (Amount :type "Float (double-precision)"))
  (set `self.CurrentManaPoints` (`KismetMathLibrary.FMax` (- (`self.CurrentManaPoints`) Amount))))

(fn `DecreaseStamina`
  (params (Amount :type "Float (double-precision)"))
  (set `self.CurrentStamina` (`KismetMathLibrary.FMax` (- (`self.CurrentStamina`) Amount))))

(fn `IncreaseHealthPoints`
  (params (Amount :type "Float (double-precision)"))
  (set `self.CurrentHealthPoints` (`KismetMathLibrary.FMin` (+ Amount (`self.CurrentHealthPoints`)) (`self.MaxHealthPoints`))))

(fn `IncreaseManaPoints`
  (params (Amount :type "Float (double-precision)"))
  (set `self.CurrentManaPoints` (`KismetMathLibrary.FMin` (+ Amount (`self.CurrentManaPoints`)) (`self.MaxManaPoints`))))

(fn `IncreaseStamina`
  (params (Amount :type "Float (double-precision)"))
  (set `self.CurrentStamina` (`KismetMathLibrary.FMin` (+ Amount (`self.CurrentStamina`)) (`self.MaxStamina`))))